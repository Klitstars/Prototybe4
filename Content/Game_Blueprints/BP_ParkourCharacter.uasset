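; BP_ParkourCharacter is a player character with movement and look input, double jump, timed slide and forward dash.
; A ParkourMovement component receives jump, landing and movement-mode events, and landing or wall contact resets the jump count.
; Sliding temporarily shrinks the capsule, while dashing sweeps along a timeline toward the camera trace's end.
; Each dash also raises an Intensity value that decays on Tick and drives post-process blend weight, with debug drawing and printing active.
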(event `InputAxis|Forward_Backward`
  (params (AxisValue :type "Float (single-precision)"))
  ;[1 1 1] Basic Movement
  (`self.AddMovementInput` (`KismetMathLibrary.GetForwardVector` (`self.GetControlRotation`)) AxisValue))

(event `InputAxis|Look_Left_Right`
  (params (AxisValue :type "Float (single-precision)"))
  ;[1 1 1] Rotation
  (`self.AddControllerYawInput` AxisValue))

(event `InputAxis|Left_Right`
  (params (AxisValue :type "Float (single-precision)"))
  ;[1 1 1] Basic Movement
  (`self.AddMovementInput` (`KismetMathLibrary.GetRightVector` (`self.GetControlRotation`)) AxisValue))

(event `InputAxis|Look_Up_Down`
  (params (AxisValue :type "Float (single-precision)"))
  ;[1 1 1] Rotation
  (`self.AddControllerPitchInput` AxisValue))

(event `InputAction|Jump`
  (params (Key :type "Key Structure"))
  ;[1 1 1] Jump and DoubleJump
  (:`Pressed`
    (bind _counter (`/Engine/EditorBlueprintResources/StandardMacros.Do N` 2 :!label _label)
      (:`Exit`
        (switch `int` _counter
          (:`1`
            (`self.LaunchCharacter` (0.0 0.0 1200.0)))
          (:`2`
            (`self.LaunchCharacter` (0.0 0.0 1500.0))))
        (`/Game/Game_Blueprints/ParkourMovement.Jump` (`self.ParkourMovement`)))))
  (:`Released`
    (`self.StopJumping`)))

(event `self.ReceiveBeginPlay`
  ;[1 1 1] WallParkour
  (`|ExecutionSequence`
    (:`then_0`
      (`MovementComponent.SetPlaneConstraintEnabled` (`self.CharacterMovement`) true))
    (:`then_1`
      (`/Game/Game_Blueprints/ParkourMovement.Initialize` (`self.ParkourMovement`) self))
    (:`then_2`
      (bind _returnvalue (`GameplayStatics.GetActorOfClass` "/Script/Engine.PostProcessVolume"))
      (set `self.PostProcess` _returnvalue))))

(event `self.K2_OnMovementModeChanged`
  (params (PrevMovementMode :type "EMovementMode Enum" :default "MOVE_None") (NewMovementMode :type "EMovementMode Enum" :default "MOVE_None") (PrevCustomMode :type Byte) (NewCustomMode :type Byte))
  (`/Game/Game_Blueprints/ParkourMovement.MovementChanged` (`self.ParkourMovement`) PrevMovementMode NewMovementMode))

(event `self.OnLanded`
  (params (Hit :type "HitResult Structure (by ref)"))
  ;[1 1 1] Jump and DoubleJump
  (`/Game/Game_Blueprints/ParkourMovement.Land` (`self.ParkourMovement`))
  (goto _label :!via `Reset`))

(event `OnWall`
  ;[1 1 1] Jump and DoubleJump
  (goto _label :!via `Reset`))

(event `Key|C`
  (params (Key :type "Key Structure"))
  (bind _mesh (`self.Mesh`))
  (bind _mesh_2 (`self.Mesh`))
  ;[1 1 1] Sliding
  (:`Pressed`
    (if (and (> (`KismetMathLibrary.VSize` (`MovementComponent.Velocity` (`self.CharacterMovement`))) 10.0) (not (`NavMovementComponent.IsFalling` (`self.CharacterMovement`))))
      (`/Engine/EditorBlueprintResources/StandardMacros.DoOnce` false :!label _label_2
        (:`Completed`
          (`CapsuleComponent.SetCapsuleHalfHeight` (`self.CapsuleComponent`) 20.0 true)
          (`SceneComponent.K2_SetWorldLocation` _mesh_2 (+ (`SceneComponent.K2_GetComponentLocation` _mesh_2) (0.0 0.0 50.0)) false false)
          (`KismetSystemLibrary.Delay` 1.0)
          (`CapsuleComponent.SetCapsuleHalfHeight` (`self.CapsuleComponent`) 88.0 true)
          (`SceneComponent.K2_SetWorldLocation` _mesh (- (`SceneComponent.K2_GetComponentLocation` _mesh) (0.0 0.0 50.0)) false false)
          (goto _label_2 :!via `Reset`))))))

(event `InputAction|Dash`
  (params (Key :type "Key Structure"))
  (bind _camera (`self.Camera`))
  (bind _returnvalue (`SceneComponent.K2_GetComponentLocation` _camera))
  ;[1 1 1] Dashing
  (:`Pressed`
    (bind _outhit (`KismetSystemLibrary.LineTraceSingle` :`Start` _returnvalue :`End` (+ _returnvalue (* (`SceneComponent.GetForwardVector` _camera) (`self.DashLength`))) :`TraceChannel` "TraceTypeQuery1" :`DrawDebugType` "Persistent"))
    (set `self.DashLocation` (`.TraceEnd` (`GameplayStatics.BreakHitResult` _outhit)))
    (set `self.PlayerLocation` (`self.K2_GetActorLocation`))
    (`self.DashMovement`)))

(event `DashMovement`
  ;[1 1 1] Dashing
  (bind (_direction _alpha) (`Timeline|Alpha` :!via `PlayFromStart`)
    (:`Update`
      (`self.K2_SetActorLocation` (`KismetMathLibrary.VLerp` (`self.PlayerLocation`) (`self.DashLocation`) _alpha) true))))

(event `InputAction|Dash`
  (params (Key :type "Key Structure"))
  ;[1 1 1] Intensity
  (:`Pressed`
    (set `self.Intensity` (+ (`self.Intensity`) 0.2))))

(event `self.ReceiveTick`
  (params (DeltaSeconds :type "Float (single-precision)"))
  ;[1 1 1] Intensity
  (`|ExecutionSequence`
    (:`then_1`
      (set `self.IntensityChange` -0.1))
    (:`then_2`
      (set `self.Intensity` (`KismetMathLibrary.FClamp` (+ (`self.Intensity`) (* (`self.IntensityChange`) DeltaSeconds)) 0.0 (`self.MaxIntensity`))))
    (:`then_3`
      (set `PostProcessVolume.BlendWeight` (`self.Intensity`) (`self.PostProcess`)))
    (:`then_4`
      (`KismetSystemLibrary.PrintString` (`KismetStringLibrary.Conv_DoubleToString` (`self.Intensity`)) true true (struct :`G` 0.66 :`B` 1.0 :`A` 1.0) 0.0))))

(fn `UserConstructionScript`)